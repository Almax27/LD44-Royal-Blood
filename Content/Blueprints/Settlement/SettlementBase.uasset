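; Base settlement actor that holds capped resources, binds a widget to itself and visualises its population.
; Each logic tick hands population gain out one unit at a time across all settlements, ordered by a single bubble pass on distance.
; Resource additions return overflow and set a dirty flag, which post-tick turns into a state-changed call.
; Every frame, static mesh components scale in or out along a curve to match the population fill ratio.
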(event `self.ReceiveBeginPlay`
  (bind _assettlement_widget (cast `/Game/Blueprints/UI/SettlementWidget` (`WidgetComponent.GetUserWidgetObject` (`self.Widget`))))
  (`/Game/Blueprints/UI/SettlementWidget.BindToSettlement` _assettlement_widget self)
  (`self.InitPopulationVisualisation`))

(event `self.ReceiveTick`
  (params (DeltaSeconds :type "Float (single-precision)"))
  (`self.TickPopulationVisualisation` DeltaSeconds))

(fn `AddResource`
  (params (Type :type "/Game/Blueprints/Gameplay/ResourceTypeEnum Enum" :default "NewEnumerator2") (Value :type Integer))
  (returns (Remainder :type Integer))
  (locals (AmountRemaining :type Integer))
  (bind _value (`local.Value`))
  (bind (_value_2 _returnvalue) (`BlueprintMapLibrary.Map_Find` (`self.ResourceStateMap`) Type))
  (bind (_amount _capacity _gain) (break `/Game/Blueprints/Gameplay/ResourceState` _value_2))
  (bind _returnvalue_2 (`KismetMathLibrary.Max` (- _value (`local.AmountRemaining`))))
  (if _returnvalue
    (bind _output_get (set `local.AmountRemaining` (- _capacity _amount)))
    (if (> _output_get 0)
      (`BlueprintMapLibrary.Map_Add` (`self.ResourceStateMap`) Type (make `/Game/Blueprints/Gameplay/ResourceState` (+ (`KismetMathLibrary.Min` (`local.AmountRemaining`) (`local.Value`)) _amount) _capacity _gain))
      (set `self.IsDirty` (!= _value _returnvalue_2))
      (return _returnvalue_2)
      (else
        _)))
  (return Value))

(fn `GetSettlementsByDistance`
  (returns (Settlements :type "Array of /Game/Blueprints/Settlement/SettlementBase Object Reference"))
  (locals (SortedSettlements :type "Array of /Game/Blueprints/Settlement/SettlementBase Object Reference"))
  (bind _sortedsettlements (`local.SortedSettlements`))
  (bind _outactors (`GameplayStatics.GetAllActorsOfClass` "SettlementBase_C"))
  (bind _output_get (set `local.SortedSettlements` _outactors))
  (bind _returnvalue (`KismetArrayLibrary.Array_LastIndex` _output_get))
  (for _index (range 1 (+ _returnvalue 1))
    (bind _returnvalue_2 (- _returnvalue _index))
    (if (< (`self.GetDistanceTo` (`|GetArrayItem` _sortedsettlements (+ _returnvalue_2 1))) (`self.GetDistanceTo` (`|GetArrayItem` _sortedsettlements _returnvalue_2)))
      (`KismetArrayLibrary.Array_Swap` (`local.SortedSettlements`) (+ _returnvalue_2 1) _returnvalue_2)))
  (return (`local.SortedSettlements`)))

(fn `InitPopulationVisualisation`
  (for _array_element (`self.K2_GetComponentsByClass` "/Script/Engine.StaticMeshComponent")
    (`BlueprintMapLibrary.Map_Add` (`self.PopulationState`) _array_element)))

(fn `PostTickGamelogic`
  (if (`self.IsDirty`)
    (set `self.IsDirty` false)
    (`self.SettlementStateChanged` self)))

(fn `TickGameLogic`
  (locals (Remaining :type Integer) (Consumed :type Boolean :default true))
  (bind (_value _returnvalue) (`BlueprintMapLibrary.Map_Find` (`self.ResourceStateMap`) "NewEnumerator1"))
  ;[1 1 1] Distribute population gain to other settlements
  (bind _settlements (`self.GetSettlementsByDistance`))
  (if _returnvalue
    (set `local.Remaining` (`.Gain_14_69DF3AB54B2428EB727668AB5A30231F` (break `/Game/Blueprints/Gameplay/ResourceState` _value)))
    (while (and (> (`local.Remaining`) 0) (`local.Consumed`))
      (set `local.Consumed` false)
      (for _array_element _settlements
        (bind _remainder (`self.AddResource` _array_element "NewEnumerator1" 1))
        (bind _result (`/Engine/EditorBlueprintResources/StandardMacros.DecrementInt` (`local.Remaining`))
          (:`  `
            (`|ExecutionSequence`
              (:`then_0`
                (bind _returnvalue_2 (== _remainder 0))
                (if _returnvalue_2
                  _))
              (:`then_1`
                (set `local.Remaining` (+ _result _remainder))
                (if (> (`local.Remaining`) 0)
                  (set `local.Consumed` _returnvalue_2)
                  (else
                    (break)))))))))))

(fn `TickPopulationVisualisation`
  (params (DeltaTIme :type "Float (double-precision)"))
  (locals (EnabledIndex :type Integer) (State :type "Float (double-precision)"))
  (bind _populationstate (`self.PopulationState`))
  (bind _deltatime (`local.DeltaTIme`))
  (bind (_value _returnvalue) (`BlueprintMapLibrary.Map_Find` (`self.ResourceStateMap`) "NewEnumerator1"))
  (bind (_amount _capacity) (break `/Game/Blueprints/Gameplay/ResourceState` _value))
  (`|ExecutionSequence`
    (:`then_0`
      (if _returnvalue
        (set `local.EnabledIndex` (`KismetMathLibrary.FFloor` (* (`BlueprintMapLibrary.Map_Length` (`self.PopulationState`)) (/ (`KismetMathLibrary.Conv_IntToDouble` _amount) (`KismetMathLibrary.Conv_IntToDouble` _capacity)))))
        (bind _keys (`BlueprintMapLibrary.Map_Keys` (`self.PopulationState`)))
        (for (_array_element _array_index) _keys
          (bind _value_2 (`BlueprintMapLibrary.Map_Find` (`self.PopulationState`) _array_element))
          (set `local.State` _value_2)
          (if (< _array_index (`local.EnabledIndex`))
            (`BlueprintMapLibrary.Map_Add` (`self.PopulationState`) _array_element (`KismetMathLibrary.FClamp` (+ _value_2 _deltatime)))
            (if (== (`local.State`) 0.0)
              _)
            (else
              (`BlueprintMapLibrary.Map_Add` (`self.PopulationState`) _array_element (`KismetMathLibrary.FClamp` (- _value_2 _deltatime)))
              (if (== (`local.State`) 1.0)
                _))))
        (else
          ;[1 1 1] Reset all
          (bind _keys_2 (`BlueprintMapLibrary.Map_Keys` _populationstate))
          (for _array_element_2 _keys_2
            (`BlueprintMapLibrary.Map_Add` _populationstate _array_element_2)))))
    (:`then_1`
      (bind _keys_3 (`BlueprintMapLibrary.Map_Keys` (`self.PopulationState`)))
      (for _array_element_3 _keys_3
        (`SceneComponent.SetRelativeScale3D` _array_element_3 (`CurveVector.GetVectorValue` (`self.PopulationAnimCurve`) (`BlueprintMapLibrary.Map_Find` (`self.PopulationState`) _array_element_3)))))))

(fn `UserConstructionScript`)