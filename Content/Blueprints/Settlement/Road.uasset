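; Settlement road actor that lays a chain of deformed spline meshes along its spline in the construction script.
; Each segment's length comes from the chosen mesh's X bounds, with meshes cycled or picked from a seeded random stream, until the next would overrun the spline.
; UpdateSplineMesh matches position, tangent, roll and scale to the spline, updating once per segment.
; Flags can pause rebuilding or clear existing components, which are otherwise gathered for reuse.
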(fn `GetNextMesh`
  (returns (NewParam :type "StaticMesh Object Reference"))
  (bind _meshes (`self.Meshes`))
  (bind _returnvalue (`KismetArrayLibrary.Array_Length` (`self.Meshes`)))
  (if (> _returnvalue 0)
    (if (`self.RandomiseMeshes`)
      (return (`|GetArrayItem` _meshes (`KismetMathLibrary.RandomIntegerInRangeFromStream` 0 (`KismetArrayLibrary.Array_LastIndex` _meshes) (`self.RandomStream`))))
      (else
        (bind _result (`/Engine/EditorBlueprintResources/StandardMacros.IncrementInt` (`self.LastMeshIndex`))
          (:`  `
            (return (`|GetArrayItem` (`self.Meshes`) (mod _result _returnvalue)))))))))

(fn `UpdateSplineMesh`
  (params (SplineMesh :type "SplineMeshComponent Object Reference") (StaticMesh :type "StaticMesh Object Reference") (FromDistance :type "Float (double-precision)") (ToDistance :type "Float (double-precision)"))
  (bind _spline (`self.Spline`))
  (bind _spline_2 (`self.Spline`))
  (bind _spline_3 (`self.Spline`))
  (`StaticMeshComponent.SetStaticMesh` SplineMesh StaticMesh)
  (`SplineMeshComponent.SetStartAndEnd` SplineMesh (`SplineComponent.GetLocationAtDistanceAlongSpline` _spline FromDistance "Local") (`SplineComponent.GetTangentAtDistanceAlongSpline` _spline FromDistance "Local") (`SplineComponent.GetLocationAtDistanceAlongSpline` _spline ToDistance "Local") (`SplineComponent.GetTangentAtDistanceAlongSpline` _spline ToDistance "Local") false)
  (`SplineMeshComponent.SetStartRoll` SplineMesh (.roll (`SplineComponent.GetRotationAtDistanceAlongSpline` _spline_2 FromDistance "Local")) false)
  (`SplineMeshComponent.SetEndRoll` SplineMesh (.roll (`SplineComponent.GetRotationAtDistanceAlongSpline` _spline_2 ToDistance "Local")) false)
  (`SplineMeshComponent.SetStartScale` SplineMesh (`KismetMathLibrary.Conv_VectorToVector2D` (`SplineComponent.GetScaleAtDistanceAlongSpline` _spline_3 FromDistance)) false)
  (`SplineMeshComponent.SetEndScale` SplineMesh (`KismetMathLibrary.Conv_VectorToVector2D` (`SplineComponent.GetScaleAtDistanceAlongSpline` _spline_3 ToDistance)) false)
  (`SplineMeshComponent.UpdateMesh` SplineMesh))

(fn `UserConstructionScript`
  (locals (NextIndex :type Integer) (Mesh :type "StaticMesh Object Reference") (MeshComponents :type "Array of SplineMeshComponent Object Reference") (FromDistance :type "Float (double-precision)") (ToDistance :type "Float (double-precision)") (Continue :type Boolean :default true))
  (bind _meshcomponents (`local.MeshComponents`))
  (bind _meshcomponents_2 (`local.MeshComponents`))
  (`KismetMathLibrary.ResetRandomStream` (`self.RandomStream`))
  (if (not (`self.PauseRebuild`))
    (set `self.LastMeshIndex` 0)
    (set `local.MeshComponents` (`self.K2_GetComponentsByClass` "/Script/Engine.SplineMeshComponent"))
    (`|ExecutionSequence`
      (:`then_0`
        ;[1 1 1] Clear
        (if (`self.ClearOnNextRebuild`)
          (for _array_element _meshcomponents
            (`ActorComponent.K2_DestroyComponent` _array_element))
          (`KismetArrayLibrary.Array_Clear` _meshcomponents)))
      (:`then_1`
        (while (`local.Continue`)
          (bind _output_get (set `local.Mesh` (`self.GetNextMesh`)))
          (set `local.FromDistance` (`local.ToDistance`))
          (bind (_min _max) (break `Box` (`StaticMesh.GetBoundingBox` _output_get)))
          (bind _output_get_2 (set `local.ToDistance` (+ (`local.FromDistance`) (- (.x _max) (.x _min)))))
          (bind _output_get_3 (set `local.Continue` (< _output_get_2 (`SplineComponent.GetSplineLength` (`self.Spline`)))))
          (if _output_get_3
            (if (not (`KismetArrayLibrary.Array_IsValidIndex` (`local.MeshComponents`) (`local.NextIndex`)))
              (bind _returnvalue (`AddComponent|NODE_AddSplineMeshComponent-4`))
              (bind _returnvalue_2 (`KismetArrayLibrary.Array_Add` _meshcomponents_2 _returnvalue))
              (set `local.NextIndex` (+ _returnvalue_2 1)))
            (`self.UpdateSplineMesh` (`|GetArrayItem` _meshcomponents_2 _returnvalue_2) (`local.Mesh`) (`local.FromDistance`) (`local.ToDistance`))))))))