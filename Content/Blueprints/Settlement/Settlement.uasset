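; Settlement actor with a type (empty, farm, town or city) that holds population and spawns a matching visualisation whenever its type changes.
; Type data comes from RBGameMode, and a widget binds to the actor at BeginPlay.
; TickGameLogic hands population gain out one unit at a time across settlements, ordered by a single distance bubble pass.
; AddPopulation clamps to capacity and returns overflow, setting a dirty flag that PostTickGamelogic turns into a state-changed notification.
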(event `self.ReceiveBeginPlay`
  (if (`KismetSystemLibrary.IsStandalone`)
    (`self.SetSettlementType` (`self.DebugSettlementType`)))
  (`|ExecutionSequence`
    (:`then_0`
      (bind _assettlement_widget (cast `/Game/Blueprints/UI/SettlementWidget` (`WidgetComponent.GetUserWidgetObject` (`self.Widget`))))
      (`/Game/Blueprints/UI/SettlementWidget.BindToSettlement` _assettlement_widget self))
    (:`then_1`
      (bind _asrbgame_mode (cast `/Game/Blueprints/RBGameMode` (`GameplayStatics.GetGameMode`)))
      (add `/Game/Blueprints/RBGameMode.FlowStateChanged` _asrbgame_mode (delegate `FlowStateChanged`)))))

(event `FlowStateChanged`
  (params (State :type "/Game/Blueprints/Gameplay/GameFlowState Enum" :default "NewEnumerator0")))

(event `SettlementTypeChanged`
  (bind _settlementvisualisation (`self.SettlementVisualisation`))
  (`|ExecutionSequence`
    (:`then_0`
      ;[1 1 1] Cleanup existing Visualisaiton
      (`/Engine/EditorBlueprintResources/StandardMacros.IsValid` _settlementvisualisation
        (:`Is Valid`
          (`self.K2_DestroyActor` _settlementvisualisation))))
    (:`then_1`
      (bind _returnvalue (`|SpawnActorFromClass` (castclass `/Game/Blueprints/Settlement/SettlementVisualisation` (select `/Game/Blueprints/Gameplay/SettlementType` (`self.SettlementType`) :`NewEnumerator4` "/Game/Blueprints/Settlement/SettlementVisualisation.SettlementVisualisation_C" :`NewEnumerator1` "/Game/Blueprints/Settlement/Visualisations/FarmA.FarmA_C" :`NewEnumerator2` "/Game/Blueprints/Settlement/Visualisations/TownA.TownA_C" :`NewEnumerator3` "/Game/Blueprints/Settlement/Visualisations/CityA.CityA_C" :!type "Actor Class Reference") :!pure true) (`self.GetTransform`) "Undefined" "OverrideRootScale" null self null))
      (bind _assettlement_visualisation (cast `/Game/Blueprints/Settlement/SettlementVisualisation` _returnvalue)
        (:`then`
          (set `self.SettlementVisualisation` _assettlement_visualisation))
        (:`CastFailed`
          (`KismetSystemLibrary.PrintString` "Invalid settlement visualisation" true true (struct :`R` 1.0 :`A` 1.0) 10.0))))
    (:`then_2`
      (`self.SettlementStateChanged` self))))

(fn `AddPopulation`
  (params (Value :type Integer))
  (returns (Remainder :type Integer))
  (locals (DesiredPopulation :type Integer))
  (bind _output_get (set `local.DesiredPopulation` (+ (`self.Population`) Value)))
  (bind _returnvalue (`KismetMathLibrary.Clamp` _output_get 0 (`.PopulationCapacity_10_1AE78F75454F259B41A03F80F2EB7122` (break `/Game/Blueprints/Gameplay/SettlementData` (`self.GetSettlementData`)))))
  (set `self.IsDirty` (!= (`self.Population`) _returnvalue))
  (set `self.Population` _returnvalue)
  (return (- (`local.DesiredPopulation`) (`self.Population`))))

(fn `GetSettlementData`
  (returns (SettlementData :type "/Game/Blueprints/Gameplay/SettlementData Structure"))
  (bind _asrbgame_mode (cast `/Game/Blueprints/RBGameMode` (`GameplayStatics.GetGameMode`))
    (:`then`
      (return (`/Game/Blueprints/RBGameMode.GetSettlementData` _asrbgame_mode (`self.SettlementType`))))
    (:`CastFailed`
      (return))))

(fn `GetSettlementName`
  (returns (Name :type Text))
  (bind (_value _returnvalue) (`BlueprintMapLibrary.Map_Find` (`self.Names`) (`self.SettlementType`)))
  (if _returnvalue
    (return _value)
    (else
      (return (`.Name_2_D5BA1DC948D02619E8C605AFD9946735` (break `/Game/Blueprints/Gameplay/SettlementData` (`self.GetSettlementData`)))))))

(fn `GetSettlementsByDistance`
  (returns (Settlements :type "Array of /Game/Blueprints/Settlement/Settlement Object Reference"))
  (locals (SortedSettlements :type "Array of /Game/Blueprints/Settlement/Settlement Object Reference"))
  (bind _sortedsettlements (`local.SortedSettlements`))
  (bind _outactors (`GameplayStatics.GetAllActorsOfClass` "Settlement_C"))
  (bind _output_get (set `local.SortedSettlements` _outactors))
  (bind _returnvalue (`KismetArrayLibrary.Array_LastIndex` _output_get))
  (for _index (range 1 (+ _returnvalue 1))
    (bind _returnvalue_2 (- _returnvalue _index))
    (if (< (`self.GetDistanceTo` (`|GetArrayItem` _sortedsettlements (+ _returnvalue_2 1))) (`self.GetDistanceTo` (`|GetArrayItem` _sortedsettlements _returnvalue_2)))
      (`KismetArrayLibrary.Array_Swap` (`local.SortedSettlements`) (+ _returnvalue_2 1) _returnvalue_2)))
  (return (`local.SortedSettlements`)))

(fn `PostTickGamelogic`
  (if (`self.IsDirty`)
    (set `self.IsDirty` false)
    (`self.SettlementStateChanged` self)))

(fn `SetSettlementType`
  (params (Type :type "/Game/Blueprints/Gameplay/SettlementType Enum" :default "NewEnumerator4"))
  (if (`|EnumInequality` Type (`self.SettlementType`))
    (set `self.SettlementType` Type)
    (`self.SettlementTypeChanged`)))

(fn `TickGameLogic`
  (locals (Remaining :type Integer) (Consumed :type Boolean :default true))
  ;[1 1 1] Distribute population gain to other settlements
  (bind _settlements (`self.GetSettlementsByDistance`))
  (set `local.Remaining` (`.PopulationGain_11_F62F3AF646DBFF51E7C37A8C275CBFF0` (break `/Game/Blueprints/Gameplay/SettlementData` (`self.GetSettlementData`))))
  (while (and (> (`local.Remaining`) 0) (`local.Consumed`))
    (set `local.Consumed` false)
    (for _array_element _settlements
      (bind _remainder (`self.AddPopulation` _array_element 1))
      (bind _result (`/Engine/EditorBlueprintResources/StandardMacros.DecrementInt` (`local.Remaining`))
        (:`  `
          (`|ExecutionSequence`
            (:`then_0`
              (bind _returnvalue (== _remainder 0))
              (if _returnvalue
                _))
            (:`then_1`
              (set `local.Remaining` (+ _result _remainder))
              (if (> (`local.Remaining`) 0)
                (set `local.Consumed` _returnvalue)
                (else
                  (break))))))))))

(fn `UserConstructionScript`
  (`TextRenderComponent.K2_SetText` (`self.EditorText`) (`KismetTextLibrary.Conv_StringToText` (`|GetEnumeratorNameAsString` (`self.SettlementType`)))))