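; TownSettlement is a settlement Blueprint for a town that seeds its resource state when play begins.
; After calling its parent, BeginPlay casts the game mode to RBGameMode and copies GameBalance.TownStartingResources into ResourceStateMap, so starting values come from the game mode's balance data.
; If the cast fails, the map is left untouched.
; The construction script only calls its parent, and the Tick and overlap events are disabled.
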(event `self.ReceiveBeginPlay`
  (`parent.ReceiveBeginPlay`)
  (bind _asrbgame_mode (cast `/Game/Blueprints/RBGameMode` (`GameplayStatics.GetGameMode`)))
  (set `self.ResourceStateMap` (`/Game/Blueprints/Balance/GameBalance.TownStartingResources` (`/Game/Blueprints/RBGameMode.GameBalance` _asrbgame_mode))))

(fn `UserConstructionScript`
  (`parent.UserConstructionScript`))