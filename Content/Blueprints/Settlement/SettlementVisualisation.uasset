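; Settlement visual actor that shows population by scaling its static mesh buildings in and out.
; On BeginPlay it gathers every static mesh component as a building, each with a zeroed animation state.
; Each Tick, the population-to-capacity ratio sets how many buildings are enabled.
; Their states move toward one or zero over about a second, driving relative scale through a vector curve.
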(event `self.ReceiveBeginPlay`
  (`self.InitPopulationVisualisation`))

(event `self.ReceiveTick`
  (params (DeltaSeconds :type "Float (single-precision)"))
  (`self.TickPopulationVisualisation` DeltaSeconds))

(fn `GetSettlementData`
  (returns (SettlementData :type "/Game/Blueprints/Gameplay/SettlementData Structure"))
  (bind _settlement (`self.Settlement`))
  (`/Engine/EditorBlueprintResources/StandardMacros.IsValid` _settlement
    (:`Is Valid`
      (return (`/Game/Blueprints/Settlement/Settlement.GetSettlementData` _settlement)))
    (:`Is Not Valid`
      (return))))

(fn `InitPopulationVisualisation`
  (`KismetArrayLibrary.Array_Clear` (`self.Buildings`))
  (`KismetArrayLibrary.Array_Clear` (`self.BuildingStates`))
  (for _array_element (`self.K2_GetComponentsByClass` "/Script/Engine.StaticMeshComponent")
    (`KismetArrayLibrary.Array_Add` (`self.Buildings`) _array_element)
    (`KismetArrayLibrary.Array_Add` (`self.BuildingStates`)))
  (`self.TickPopulationVisualisation` 0.0 true))

(fn `TickPopulationVisualisation`
  (params (DeltaTIme :type "Float (double-precision)") (ForceUpdate :type Boolean))
  (locals (EnabledIndex :type Integer) (State :type "Float (double-precision)"))
  (if (> (`KismetArrayLibrary.Array_Length` (`self.Buildings`)) 0)
    (set `local.EnabledIndex` (`KismetMathLibrary.FFloor` (* (`KismetArrayLibrary.Array_Length` (`self.BuildingStates`)) (/ (`KismetMathLibrary.Conv_IntToDouble` (`/Game/Blueprints/Settlement/Settlement.Population` (`self.Settlement`))) (`KismetMathLibrary.Conv_IntToDouble` (`.PopulationCapacity_10_1AE78F75454F259B41A03F80F2EB7122` (break `/Game/Blueprints/Gameplay/SettlementData` (`self.GetSettlementData`))))))))
    (for _index (range (+ (`KismetArrayLibrary.Array_LastIndex` (`self.Buildings`)) 1))
      (set `local.State` (`|GetArrayItem` (`self.BuildingStates`) _index))
      (if (< _index (`local.EnabledIndex`))
        (set `local.State` (`KismetMathLibrary.FClamp` (+ (`local.State`) (`local.DeltaTIme`))))
        (if (or (!= (`local.State`) 1.0) (`local.ForceUpdate`))
          (`SceneComponent.SetRelativeScale3D` (`|GetArrayItem` (`self.Buildings`) _index) (`CurveVector.GetVectorValue` (`self.PopulationAnimCurve`) (`local.State`)) :!label _label)
          (`KismetArrayLibrary.Array_Set` (`self.BuildingStates`) _index (`local.State`)))
        (else
          (set `local.State` (`KismetMathLibrary.FClamp` (- (`local.State`) (`local.DeltaTIme`))))
          (if (or (!= (`local.State`) 0.0) (`local.ForceUpdate`))
            (goto _label)))))))

(fn `UserConstructionScript`)