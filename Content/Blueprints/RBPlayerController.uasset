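; Player controller that possesses the level's CameraSplinePawn and handles mouse-drag camera scrolling and game-flow input.
; Flow state changes from RBGameMode allow scrolling only during the four seasons.
; Drags project the cursor onto a ground plane to derive velocity, which eases out after release and moves the pawn.
; Any key advances Splash, Win and Loss screens; non-distribution builds add debug keys for flow states and settlement actions.
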(event `self.ReceiveBeginPlay`
  (`WidgetBlueprintLibrary.SetInputMode_GameAndUIEx` self null "DoNotLock" false)
  (bind _outactors (`GameplayStatics.GetAllActorsOfClass` "/Game/Blueprints/Camera/CameraSplinePawn.CameraSplinePawn_C"))
  (if (`KismetArrayLibrary.Array_IsValidIndex` _outactors)
    (`self.Possess` (`|GetArrayItem` _outactors))
    (bind _asrbgame_mode (cast `/Game/Blueprints/RBGameMode` (`GameplayStatics.GetGameMode`)))
    (add `/Game/Blueprints/RBGameMode.FlowStateChanged` _asrbgame_mode (delegate `FlowStateChanged`))
    (`self.FlowStateChanged` (`/Game/Blueprints/RBGameMode.FlowState` _asrbgame_mode))
    (else
      (`KismetSystemLibrary.PrintString` "Scene must contain a camera spline!" true true (struct :`R` 1.0 :`A` 1.0) 10.0))))

(event `FlowStateChanged`
  (params (State :type "/Game/Blueprints/Gameplay/GameFlowState Enum" :default "NewEnumerator8"))
  (set `self.CanScroll` (select `/Game/Blueprints/Gameplay/GameFlowState` State :`NewEnumerator2` true :`NewEnumerator3` true :`NewEnumerator4` true :`NewEnumerator5` true)))

(event `self.ReceiveTick`
  (params (DeltaSeconds :type "Float (single-precision)"))
  (`|ExecutionSequence`
    (:`then_0`
      (if (`self.Scrolling`)
        (bind _returnvalue (`WidgetLayoutLibrary.GetMousePositionOnViewport`))
        (set `self.MouseVelocity` (/ (* (.y (- (`self.GetWorldPosition` _returnvalue) (`self.GetWorldPosition` (`self.LastMousePosition`)))) -1.0) DeltaSeconds))
        (set `self.LastMousePosition` _returnvalue)
        (else
          (set `self.MouseVelocity` (`KismetMathLibrary.FInterpTo` (`self.MouseVelocity`) 0.0 DeltaSeconds 5.0)))))
    (:`then_1`
      (if (not (`KismetMathLibrary.NearlyEqual_FloatFloat` (`self.MouseVelocity`) 0.0 0.001))
        (bind _ascamera_spline_pawn (cast `/Game/Blueprints/Camera/CameraSplinePawn` (`self.K2_GetPawn`)))
        (`/Game/Blueprints/Camera/CameraSplinePawn.AddWorldPosition` _ascamera_spline_pawn (* (`self.MouseVelocity`) DeltaSeconds))))))

(event `Key|LeftMouseButton`
  (params (Key :type "Key Structure"))
  (:`Pressed`
    (if (`self.CanScroll`)
      (set `self.Scrolling` true)
      (bind _returnvalue (`WidgetLayoutLibrary.GetMousePositionOnViewport`))
      (set `self.LastMousePosition` _returnvalue)))
  (:`Released`
    (set `self.Scrolling` false)))

(event `Key|R`
  (params (Key :type "Key Structure"))
  (:`Pressed`
    (`self.ExecDebug`
      (:`Out`
        (`/Game/Blueprints/RBGameMode.GotoFlowState` (cast `/Game/Blueprints/RBGameMode` (`GameplayStatics.GetGameMode`) :!pure true) "NewEnumerator8")))))

(event `Key|S`
  (params (Key :type "Key Structure"))
  (:`Pressed`
    (`self.ExecDebug`
      (:`Out`
        (`/Game/Blueprints/RBGameMode.GotoFlowState` (cast `/Game/Blueprints/RBGameMode` (`GameplayStatics.GetGameMode`) :!pure true) "NewEnumerator1")))))

(event `Key|One`
  (params (Key :type "Key Structure"))
  (:`Pressed`
    (`self.ExecDebug`
      (:`Out`
        (`/Game/Blueprints/RBGameMode.GotoFlowState` (cast `/Game/Blueprints/RBGameMode` (`GameplayStatics.GetGameMode`) :!pure true) "NewEnumerator2")))))

(event `Key|Two`
  (params (Key :type "Key Structure"))
  (:`Pressed`
    (`self.ExecDebug`
      (:`Out`
        (`/Game/Blueprints/RBGameMode.GotoFlowState` (cast `/Game/Blueprints/RBGameMode` (`GameplayStatics.GetGameMode`) :!pure true) "NewEnumerator3")))))

(event `Key|Three`
  (params (Key :type "Key Structure"))
  (:`Pressed`
    (`self.ExecDebug`
      (:`Out`
        (`/Game/Blueprints/RBGameMode.GotoFlowState` (cast `/Game/Blueprints/RBGameMode` (`GameplayStatics.GetGameMode`) :!pure true) "NewEnumerator4")))))

(event `Key|Four`
  (params (Key :type "Key Structure"))
  (:`Pressed`
    (`self.ExecDebug`
      (:`Out`
        (`/Game/Blueprints/RBGameMode.GotoFlowState` (cast `/Game/Blueprints/RBGameMode` (`GameplayStatics.GetGameMode`) :!pure true) "NewEnumerator5")))))

(event `Key|Five`
  (params (Key :type "Key Structure"))
  (:`Pressed`
    (`self.ExecDebug`
      (:`Out`
        (`/Game/Blueprints/RBGameMode.GotoFlowState` (cast `/Game/Blueprints/RBGameMode` (`GameplayStatics.GetGameMode`) :!pure true) "NewEnumerator6")))))

(event `Key|Six`
  (params (Key :type "Key Structure"))
  (:`Pressed`
    (`self.ExecDebug`
      (:`Out`
        (`/Game/Blueprints/RBGameMode.GotoFlowState` (cast `/Game/Blueprints/RBGameMode` (`GameplayStatics.GetGameMode`) :!pure true) "NewEnumerator7")))))

(event `Key|AnyKey` :consume false
  (params (Key :type "Key Structure"))
  (:`Pressed`
    (bind _asrbgame_mode (cast `/Game/Blueprints/RBGameMode` (`GameplayStatics.GetGameMode`)))
    (switch `/Game/Blueprints/Gameplay/GameFlowState` (`/Game/Blueprints/RBGameMode.FlowState` _asrbgame_mode)
      (:`NewEnumerator8`
        (`/Game/Blueprints/RBGameMode.GotoFlowState` _asrbgame_mode "NewEnumerator0"))
      (:`NewEnumerator6`
        (`/Game/Blueprints/RBGameMode.GotoFlowState` _asrbgame_mode "NewEnumerator1"))
      (:`NewEnumerator7`
        (`/Game/Blueprints/RBGameMode.GotoFlowState` _asrbgame_mode "NewEnumerator1")))))

(event `Key|T`
  (params (Key :type "Key Structure"))
  (:`Pressed`
    (`self.ExecDebug`
      (:`Out`
        (bind _outactors (`GameplayStatics.GetAllActorsOfClass` "/Game/Blueprints/Settlement/Settlement.Settlement_C"))
        (for _array_element _outactors
          (`/Game/Blueprints/Settlement/Settlement.TrySendTravelers` _array_element 0))))))

(event `Key|E`
  (params (Key :type "Key Structure"))
  (:`Pressed`
    (`self.ExecDebug`
      (:`Out`
        (bind _asrbgame_mode (cast `/Game/Blueprints/RBGameMode` (`GameplayStatics.GetGameMode`)))
        (`/Game/Blueprints/RBGameMode.TriggerEventOnRandomSettlement` _asrbgame_mode "NewEnumerator1")))))

(fn `GetSplineCameraPosition`
  (returns (Position :type "Float (double-precision)"))
  (bind _ascamera_spline_pawn (cast `/Game/Blueprints/Camera/CameraSplinePawn` (`self.K2_GetPawn`)))
  (return (`/Game/Blueprints/Camera/CameraSplinePawn.GetTargetCameraPosition` _ascamera_spline_pawn)))

(fn `GetWorldPosition`
  (params (Screen :type "Vector2D Structure"))
  (returns (World :type "Vector Structure"))
  (bind (_worldposition _worlddirection) (`GameplayStatics.DeprojectScreenToWorld` self Screen))
  (return (`.Intersection` (`KismetMathLibrary.LinePlaneIntersection_OriginNormal` _worldposition (+ _worldposition (* _worlddirection 10000000.0)) (0.0 0.0 0.0) (0.0 0.0 1.0)))))

(fn `SetSplineCameraPosition`
  (params (SplineCameraPosition :type "Float (double-precision)"))
  (bind _ascamera_spline_pawn (cast `/Game/Blueprints/Camera/CameraSplinePawn` (`self.K2_GetPawn`)))
  (`/Game/Blueprints/Camera/CameraSplinePawn.SetTargetCameraPosition` _ascamera_spline_pawn SplineCameraPosition))

(fn `UserConstructionScript`)