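; Fire truck vehicle that travels to a destination, ends a specific event type there if still active, then destroys itself.
; It extends a parent class, taking its speed from GameBalance and looking up one settlement type's data through RBGameMode.
; While its Wagon is valid, Tick spins the front and back wheel pairs by speed, delta time and separate radii.
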(event `self.Initialise`
  (params (GameBalance :type "/Game/Blueprints/Gameplay/GameBalance Object Reference"))
  (`parent.Initialise` GameBalance)
  (set `self.Speed` (`/Game/Blueprints/Gameplay/GameBalance.FireTruckSpeed` GameBalance)))

(event `self.ReceiveTick`
  (params (DeltaSeconds :type "Float (single-precision)"))
  (`parent.ReceiveTick` DeltaSeconds)
  (`/Engine/EditorBlueprintResources/StandardMacros.IsValid` (`self.Wagon`)
    (:`Is Valid`
      (`SceneComponent.K2_AddLocalRotation` (`self.WheelFL`) (`KismetMathLibrary.MakeRotator` 0.0 (`self.CalcWheelTurn` DeltaSeconds 31.5)) false false)
      (`SceneComponent.K2_AddLocalRotation` (`self.WheelFR`) (`KismetMathLibrary.MakeRotator` 0.0 (`self.CalcWheelTurn` DeltaSeconds 31.5)) false false)
      (`SceneComponent.K2_AddLocalRotation` (`self.WheelBL`) (`KismetMathLibrary.MakeRotator` 0.0 (`self.CalcWheelTurn` DeltaSeconds 20.0)) false false)
      (`SceneComponent.K2_AddLocalRotation` (`self.WheelBR`) (`KismetMathLibrary.MakeRotator` 0.0 (`self.CalcWheelTurn` DeltaSeconds 20.0)) false false))))

(event `self.ArrivedAtDestination`
  (`parent.ArrivedAtDestination`)
  (`|ExecutionSequence`
    (:`then_0`
      (if (`/Game/Blueprints/Settlement/Settlement.IsEventActive` (`self.Destination`) "NewEnumerator1")
        (`/Game/Blueprints/Settlement/Settlement.EndEvent` (`self.Destination`))))
    (:`then_1`
      (`self.K2_DestroyActor`))))

(fn `GetSettlementData`
  (returns (Data :type "/Game/Blueprints/Gameplay/SettlementData Structure"))
  (bind _asrbgame_mode (cast `/Game/Blueprints/RBGameMode` (`GameplayStatics.GetGameMode`))
    (:`then`
      (return (`/Game/Blueprints/RBGameMode.GetSettlementData` _asrbgame_mode "NewEnumerator4")))
    (:`CastFailed`
      (return))))

(fn `UserConstructionScript`)