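; Base-style actor that travels along a Road spline toward a Destination actor, then calls ArrivedAtDestination, which prints a message.
; BeginPlay passes game balance to an empty Initialise and converts start and destination positions to spline distances by interpolating between neighbouring points.
; Tick advances distance at constant Speed, aligning the actor to the spline tangent.
; It destroys itself on Splash, Intro, Start, Win or Loss flow states.
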(event `self.ReceiveBeginPlay`
  (`|ExecutionSequence`
    (:`then_0`
      (bind _asrbgame_mode (cast `/Game/Blueprints/RBGameMode` (`GameplayStatics.GetGameMode`)))
      (add `/Game/Blueprints/RBGameMode.FlowStateChanged` _asrbgame_mode (delegate `FlowStateChanged`))
      (`self.Initialise` (`/Game/Blueprints/RBGameMode.GameBalance` _asrbgame_mode)))
    (:`then_1`
      (set `self.Distance` (`self.GetRoadDistanceClosestToWorldPosition` (`self.K2_GetActorLocation`)))
      (set `self.TargetDistance` (`self.GetRoadDistanceClosestToWorldPosition` (`self.K2_GetActorLocation` (`self.Destination`))))
      (set `self.IsTraveling` true))))

(event `FlowStateChanged`
  (params (State :type "/Game/Blueprints/Gameplay/GameFlowState Enum" :default "NewEnumerator8"))
  (switch `/Game/Blueprints/Gameplay/GameFlowState` State
    (:`NewEnumerator8`
      _)
    (:`NewEnumerator0`
      _)
    (:`NewEnumerator1`
      _)
    (:`NewEnumerator6`
      _)
    (:`NewEnumerator7`
      _))
  (`self.K2_DestroyActor`))

(event `self.ReceiveTick`
  (params (DeltaSeconds :type "Float (single-precision)"))
  (bind _distance (`self.Distance`))
  (bind _spline (`/Game/Blueprints/Settlement/Road.Spline` (`self.Road`)))
  (if (`self.IsTraveling`)
    (`|ExecutionSequence`
      (:`then_0`
        (set `self.Distance` (`KismetMathLibrary.FInterpTo_Constant` (`self.Distance`) (`self.TargetDistance`) DeltaSeconds (`self.Speed`)))
        (`self.K2_SetActorLocationAndRotation` (`SplineComponent.GetLocationAtDistanceAlongSpline` _spline _distance "World") (`KismetMathLibrary.Conv_VectorToRotator` (`SplineComponent.GetTangentAtDistanceAlongSpline` _spline _distance "World"))))
      (:`then_1`
        (if (`KismetMathLibrary.NearlyEqual_FloatFloat` (`self.Distance`) (`self.TargetDistance`) 1.0)
          (set `self.IsTraveling` false)
          (`self.ArrivedAtDestination`))))))

(fn `ArrivedAtDestination`
  (`KismetSystemLibrary.PrintText` (`|FormatText` "{0} Arrived at {1}" (`KismetTextLibrary.Conv_StringToText` (`KismetSystemLibrary.GetDisplayName` self)) (`KismetTextLibrary.Conv_StringToText` (`KismetSystemLibrary.GetDisplayName` (`self.Destination`))))))

(fn `GetRoadDistanceClosestToWorldPosition`
  (params (WorldPosition :type "Vector Structure"))
  (returns (Distance :type "Float (double-precision)"))
  (bind _spline (`/Game/Blueprints/Settlement/Road.Spline` (`self.Road`)))
  (bind _returnvalue (`SplineComponent.FindInputKeyClosestToWorldLocation` _spline WorldPosition))
  (bind _returnvalue_2 (`KismetMathLibrary.FTrunc` _returnvalue))
  (bind _returnvalue_3 (`SplineComponent.GetDistanceAlongSplineAtSplinePoint` _spline _returnvalue_2))
  (return (+ _returnvalue_3 (* (- (`SplineComponent.GetDistanceAlongSplineAtSplinePoint` _spline (`KismetMathLibrary.FTrunc` (+ _returnvalue 1.0))) _returnvalue_3) (- _returnvalue (`KismetMathLibrary.Conv_IntToDouble` _returnvalue_2))))))

(fn `Initialise`
  (params (GameBalance :type "/Game/Blueprints/Gameplay/GameBalance Object Reference")))

(fn `UserConstructionScript`)