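; Traveler is an actor that carries one unit of population to a Destination, then destroys itself on arrival.
; It registers in the Destination's InboundTravelers count on BeginPlay and deregisters on EndPlay.
; Initialise sets Speed from GameBalance with a 10% random variance and nudges the Cube in a random horizontal direction, so travelers vary in pace and offset.
; Each event also calls its parent implementation.
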(event `self.ReceiveBeginPlay`
  (`parent.ReceiveBeginPlay`)
  (`/Engine/EditorBlueprintResources/StandardMacros.IncrementInt` (`/Game/Blueprints/Settlement/Settlement.InboundTravelers` (`self.Destination`))))

(event `self.ReceiveEndPlay`
  (params (EndPlayReason :type "EEndPlayReason Enum" :default "Destroyed"))
  (`parent.ReceiveEndPlay` EndPlayReason)
  (`/Engine/EditorBlueprintResources/StandardMacros.DecrementInt` (`/Game/Blueprints/Settlement/Settlement.InboundTravelers` (`self.Destination`))))

(event `self.ArrivedAtDestination`
  (`parent.ArrivedAtDestination`)
  (`/Game/Blueprints/Settlement/Settlement.AddPopulation` (`self.Destination`) 1)
  (`self.K2_DestroyActor`))

(event `self.Initialise`
  (params (GameBalance :type "/Game/Blueprints/Gameplay/GameBalance Object Reference"))
  (`parent.Initialise` GameBalance)
  (set `self.Speed` (* (`/Game/Blueprints/Gameplay/GameBalance.TravelerSpeed` GameBalance) (`KismetMathLibrary.RandomFloatInRange` 0.9 1.1)))
  (`SceneComponent.K2_AddRelativeLocation` (`self.Cube`) (* (`KismetMathLibrary.Normal` (`KismetMathLibrary.MakeVector` (.x (`KismetMathLibrary.RandomUnitVector`)) (.y (`KismetMathLibrary.RandomUnitVector`)))) 50.0) false false))

(fn `UserConstructionScript`)