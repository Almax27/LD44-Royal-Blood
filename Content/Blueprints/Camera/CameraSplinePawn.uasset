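; A pawn whose camera slides along a spline, driven by move-right input or by external calls.
; Input and distance deltas are divided by spline length to shift a clamped 0–1 target position, which notifies listeners when it changes.
; Each tick the current position eases toward the target with FInterpTo and places the camera at constant velocity along the spline.
; The construction script previews the camera at its starting position.
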(event `self.ReceiveBeginPlay`
  (set `self.TargetPosition` (`self.Position`)))

(event `self.ReceiveTick`
  (params (DeltaSeconds :type "Float (single-precision)"))
  (`self.TickUserInput` DeltaSeconds)
  (`self.TickCameraLocation` DeltaSeconds))

(fn `AddUserInput`
  (params (Input :type "Float (double-precision)"))
  (if (!= Input 0.0)
    (`self.SetTargetCameraPosition` (+ (`self.TargetPosition`) (/ (* Input (`self.InputSpeedCm`)) (`SplineComponent.GetSplineLength` (`self.Spline`)))))))

(fn `AddWorldPosition`
  (params (Delta :type "Float (double-precision)"))
  (`self.SetTargetCameraPosition` (+ (`self.TargetPosition`) (/ Delta (`SplineComponent.GetSplineLength` (`self.Spline`))))))

(fn `GetTargetCameraPosition`
  (returns (Position :type "Float (double-precision)"))
  (return (`self.TargetPosition`)))

(fn `SetTargetCameraPosition`
  (params (Position :type "Float (double-precision)"))
  (bind _returnvalue (`KismetMathLibrary.FClamp` Position))
  (if (!= _returnvalue (`self.TargetPosition`))
    (bind _output_get (set `self.TargetPosition` _returnvalue))
    (`self.OnTargetPositionChanged` _output_get)))

(fn `TickCameraLocation`
  (params (DeltaTime :type "Float (double-precision)"))
  (set `self.Position` (`KismetMathLibrary.FInterpTo` (`self.Position`) (`self.TargetPosition`) DeltaTime (`self.InterpSpeed`)))
  (`SceneComponent.K2_SetRelativeLocation` (`self.Camera`) (`SplineComponent.GetLocationAtTime` (`self.Spline`) (`self.Position`) "Local" true) false false))

(fn `TickUserInput`
  (params (DeltaTime :type "Float (double-precision)"))
  (`self.SetTargetCameraPosition` (+ (`self.TargetPosition`) (* DeltaTime (/ (* (`self.GetInputAxisValue`) (`self.InputSpeedCm`)) (`SplineComponent.GetSplineLength` (`self.Spline`)))))))

(fn `UserConstructionScript`
  (`SceneComponent.K2_SetRelativeLocation` (`self.Camera`) (`SplineComponent.GetLocationAtTime` (`self.Spline`) (`self.Position`) "Local" true) false false))