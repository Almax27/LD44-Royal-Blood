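; Game mode running a seasonal settlement game, won if population remains after Winter.
; A flow state machine runs splash, intro, seasons and outcome, driving timelines, camera, HUD intro and a lighting parameter collection.
; Game logic ticks blood and settlements, then totals population; a looping timer is set at BeginPlay.
; Also spawns travelers and blood-purchased caravans on the first road found, using game-balance data for costs and season length.
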(event `self.ReceiveBeginPlay`
  (bind _flowstate (`self.FlowState`))
  (bind _gamebalance (`self.GameBalance`))
  (`|ExecutionSequence`
    (:`then_0`
      (`/Engine/EditorBlueprintResources/StandardMacros.IsValid` _gamebalance
        (:`Is Valid`
          (set `self.BloodResourceState` (`/Game/Blueprints/Gameplay/GameBalance.StartingBloodResource` _gamebalance)))))
    (:`then_1`
      (bind _outactors (`GameplayStatics.GetAllActorsOfClass` "/Game/Blueprints/Settlement/Settlement.Settlement_C"))
      (`self.GatherResources` _outactors)
      (`KismetSystemLibrary.K2_SetTimerDelegate` (`|CreateDelegate` :!event `TickGameLogic`) 1.0 true))
    (:`then_2`
      (`self.Event Flow State Changed` _flowstate "NewEnumerator8")
      (`self.FlowStateChanged` _flowstate))))

(event `self.ReceiveTick`
  (params (DeltaSeconds :type "Float (single-precision)"))
  (`self.TickFlow` DeltaSeconds))

(event `Event Flow State Changed`
  (params (NewState :type "/Game/Blueprints/Gameplay/GameFlowState Enum" :default "NewEnumerator8") (PrevState :type "/Game/Blueprints/Gameplay/GameFlowState Enum" :default "NewEnumerator8"))
  (`|ExecutionSequence`
    (:`then_0`
      (switch `/Game/Blueprints/Gameplay/GameFlowState` NewState
        (:`NewEnumerator8`
          (bind _ascamera_spline_pawn (cast `/Game/Blueprints/Camera/CameraSplinePawn` (`GameplayStatics.GetPlayerPawn` 0)))
          (`/Game/Blueprints/Camera/CameraSplinePawn.SetTargetCameraPosition` _ascamera_spline_pawn 1.0))
        (:`NewEnumerator0`
          (bind _asrbhud (cast `/Game/Blueprints/RBHUD` (`PlayerController.GetHUD` (`GameplayStatics.GetPlayerController` 0)))
            (:`then`
              (`/Game/Blueprints/RBHUD.StartIntro` _asrbhud)
              (bind (_direction _cameraposition) (`Timeline|IntroTimeline` :!via `PlayFromStart` :!label _label)
                (:`Update`
                  (bind _ascamera_spline_pawn_2 (cast `/Game/Blueprints/Camera/CameraSplinePawn` (`GameplayStatics.GetPlayerPawn` 0)))
                  (`/Game/Blueprints/Camera/CameraSplinePawn.SetTargetCameraPosition` _ascamera_spline_pawn_2 _cameraposition))
                (:`Finished`
                  (`self.GotoFlowState` "NewEnumerator1" :!label _label_2)
                  (`/Game/Blueprints/RBHUD.EndIntro` _asrbhud))
                (:`Progress`
                  (`/Game/Blueprints/RBHUD.ProgressIntro` _asrbhud))))
            (:`CastFailed`
              (goto _label_2))))
        (:`NewEnumerator1`
          (`Timeline|StartTimeline` :!via `PlayFromStart` :!label _label_3
            (:`Finished`
              (`self.GotoFlowState` "NewEnumerator2"))))
        (:`NewEnumerator6`
          (`Timeline|WinTimeline` :!via `PlayFromStart` :!label _label_4
            (:`Finished`
              (`self.GotoFlowState` "NewEnumerator1"))))
        (:`NewEnumerator7`
          (`Timeline|LossTimeline` :!via `PlayFromStart` :!label _label_5
            (:`Finished`
              (`self.GotoFlowState` "NewEnumerator1"))))))
    (:`then_1`
      (switch `/Game/Blueprints/Gameplay/GameFlowState` PrevState
        (:`NewEnumerator0`
          (`|ExecutionSequence`
            (:`then_0`
              (goto _label :!via `Stop`))
            (:`then_1`
              (bind _ascamera_spline_pawn_3 (cast `/Game/Blueprints/Camera/CameraSplinePawn` (`GameplayStatics.GetPlayerPawn` 0)))
              (`/Game/Blueprints/Camera/CameraSplinePawn.SetTargetCameraPosition` _ascamera_spline_pawn_3 0.0))))
        (:`NewEnumerator1`
          (goto _label_3 :!via `Stop`))
        (:`NewEnumerator6`
          (goto _label_4 :!via `Stop`))
        (:`NewEnumerator7`
          (goto _label_5 :!via `Stop`))))
    (:`then_2`
      ;[1 1 1] Material param update
      (switch `/Game/Blueprints/Gameplay/GameFlowState` NewState
        (:`NewEnumerator0`
          _)
        (:`NewEnumerator1`
          _)
        (:`NewEnumerator2`
          _)
        (:`NewEnumerator3`
          _)
        (:`NewEnumerator4`
          _)
        (:`NewEnumerator5`
          _))
      (`KismetMaterialLibrary.SetScalarParameterValue` "/Game/Materials/EnvironmentMatParams.EnvironmentMatParams" "LightStrength" (select `/Game/Blueprints/Gameplay/GameFlowState` NewState :`NewEnumerator4` 10.0 :`NewEnumerator5` 50.0 :!type "Float (single-precision)")))))

(fn `GatherResources`
  (params (Settlements :type "Array of /Game/Blueprints/Settlement/Settlement Object Reference (by ref)"))
  (locals (TotalPopulationState :type "/Game/Blueprints/Gameplay/ResourceState Structure"))
  (bind (_amount _capacity _gain) (break `/Game/Blueprints/Gameplay/ResourceState` (`local.TotalPopulationState`)))
  (`|ExecutionSequence`
    (:`then_0`
      (for _array_element Settlements
        (bind (_amount_2 _capacity_2 _gain_2) (`/Game/Blueprints/Settlement/Settlement.GetPopulationInfo` _array_element))
        (set `local.TotalPopulationState` (make `/Game/Blueprints/Gameplay/ResourceState` (+ _amount_2 _amount) (+ _capacity_2 _capacity) (+ _gain_2 _gain))))
      (`BlueprintMapLibrary.Map_Add` (`self.ResourceStateMap`) "NewEnumerator1" (`local.TotalPopulationState`)))
    (:`then_2`
      (`self.ResourcesChanged` self))))

(fn `GetSeasonDuration`
  (returns (Duration :type "Float (double-precision)"))
  (return (`/Game/Blueprints/Gameplay/GameBalance.SeasonDuration` (`self.GameBalance`))))

(fn `GetSettlementData`
  (params (SettlementType :type "/Game/Blueprints/Gameplay/SettlementType Enum" :default "NewEnumerator4"))
  (returns (Data :type "/Game/Blueprints/Gameplay/SettlementData Structure"))
  (return (`BlueprintMapLibrary.Map_Find` (`/Game/Blueprints/Gameplay/GameBalance.SettlementDataMap` (`self.GameBalance`)) SettlementType)))

(fn `GotoFlowState`
  (params (NewState :type "/Game/Blueprints/Gameplay/GameFlowState Enum" :default "NewEnumerator8"))
  (locals (PreviousState :type "/Game/Blueprints/Gameplay/GameFlowState Enum"))
  (bind _flowstate (`self.FlowState`))
  (set `local.PreviousState` _flowstate)
  (if (`|EnumInequality` NewState _flowstate)
    (bind _output_get (set `self.FlowState` NewState))
    (set `self.FlowStateTick` 0.0)
    (`KismetSystemLibrary.PrintText` (`|FormatText` "{0} ==> {1}" (`KismetTextLibrary.Conv_StringToText` (`|GetEnumeratorNameAsString` (`local.PreviousState`))) (`KismetTextLibrary.Conv_StringToText` (`|GetEnumeratorNameAsString` (`self.FlowState`)))) true true (struct :`R` 0.625 :`G` 0.005329 :`A` 1.0) 3.0)
    (`self.Event Flow State Changed` _output_get (`local.PreviousState`))
    (`self.FlowStateChanged` _output_get)))

(fn `SpawnCaravan`
  (params (Destination :type "/Game/Blueprints/Settlement/Settlement Object Reference") (Type :type "/Game/Blueprints/Gameplay/SettlementType Enum" :default "NewEnumerator4"))
  (returns (Success :type Boolean))
  (bind _success (`self.TryPayBlood` (`.PurchaseCost_22_C44B70A740A8D8AA7AB422B9821DBA02` (break `/Game/Blueprints/Gameplay/SettlementData` (`self.GetSettlementData` Type)))))
  (if _success
    (bind _outactors (`GameplayStatics.GetAllActorsOfClass` "/Game/Blueprints/Settlement/Road.Road_C"))
    (if (`KismetArrayLibrary.Array_IsValidIndex` _outactors)
      (bind _output (`|GetArrayItem` _outactors))
      (`|SpawnActorFromClass` "/Game/Blueprints/Gameplay/Caravan.Caravan_C" (`SplineComponent.GetTransformAtSplinePoint` (`/Game/Blueprints/Settlement/Road.Spline` _output) 0 "World" false) "Undefined" "OverrideRootScale" null Type Destination _output null)
      (return true)
      (else
        (`KismetSystemLibrary.PrintString` "Map must contain a road!" true true (struct :`R` 1.0 :`B` 0.027538 :`A` 1.0))
        (return false)))
    (else
      (return false))))

(fn `SpawnTraveler`
  (params (FromDestination :type "/Game/Blueprints/Settlement/Settlement Object Reference") (ToDestination :type "/Game/Blueprints/Settlement/Settlement Object Reference"))
  (returns (Success :type Boolean))
  (bind _outactors (`GameplayStatics.GetAllActorsOfClass` "/Game/Blueprints/Settlement/Road.Road_C"))
  (if (`KismetArrayLibrary.Array_IsValidIndex` _outactors)
    (bind _output (`|GetArrayItem` _outactors))
    (`|SpawnActorFromClass` "/Game/Blueprints/Gameplay/Traveler.Traveler_C" (`SplineComponent.FindTransformClosestToWorldLocation` (`/Game/Blueprints/Settlement/Road.Spline` _output) (`self.K2_GetActorLocation` FromDestination) "World" false) "Undefined" "OverrideRootScale" null FromDestination ToDestination _output null)
    (return true)
    (else
      (`KismetSystemLibrary.PrintString` "Map must contain a road!" true true (struct :`R` 1.0 :`B` 0.027538 :`A` 1.0))
      (return false))))

(fn `TickFlow`
  (params (DeltaTime :type "Float (double-precision)"))
  (bind _duration (`self.GetSeasonDuration`))
  (set `self.FlowStateTick` (+ DeltaTime (`self.FlowStateTick`)))
  (switch `/Game/Blueprints/Gameplay/GameFlowState` (`self.FlowState`)
    (:`NewEnumerator2`
      _)
    (:`NewEnumerator3`
      _)
    (:`NewEnumerator4`
      _)
    (:`NewEnumerator5`
      _))
  ;[1 1 1] Handle Season Flow progression
  (`|ExecutionSequence`
    (:`then_0`
      (if (> (`self.FlowStateTick`) _duration)
        (set `self.FlowStateTick` (- (`self.FlowStateTick`) _duration))
        (switch `/Game/Blueprints/Gameplay/GameFlowState` (`self.FlowState`)
          (:`NewEnumerator2`
            (`self.GotoFlowState` "NewEnumerator3"))
          (:`NewEnumerator3`
            (`self.GotoFlowState` "NewEnumerator4"))
          (:`NewEnumerator4`
            (`self.GotoFlowState` "NewEnumerator5"))
          (:`NewEnumerator5`
            (if (> (`.Amount_9_597E0D8540D5D5D4E8DAD783A815F3A8` (break `/Game/Blueprints/Gameplay/ResourceState` (`BlueprintMapLibrary.Map_Find` (`self.ResourceStateMap`) "NewEnumerator1"))) 0)
              (`self.GotoFlowState` "NewEnumerator6")
              (else
                (`self.GotoFlowState` "NewEnumerator7")))))))
    (:`then_1`
      (switch `/Game/Blueprints/Gameplay/GameFlowState` (`self.FlowState`)
        (:`NewEnumerator2`
          _)
        (:`NewEnumerator3`
          _)
        (:`NewEnumerator4`
          _)
        (:`NewEnumerator5`
          _))
      (`self.UpdateSeason`))))

(fn `TickGameLogic`
  (bind _bloodresourcestate (`self.BloodResourceState`))
  (bind (_amount _capacity _gain) (break `/Game/Blueprints/Gameplay/ResourceState` _bloodresourcestate))
  (bind _outactors (`GameplayStatics.GetAllActorsOfClass` "/Game/Blueprints/Settlement/Settlement.Settlement_C"))
  (`|ExecutionSequence`
    (:`then_0`
      (setmembers `/Game/Blueprints/Gameplay/ResourceState` :`StructRef` _bloodresourcestate :`Amount` (`KismetMathLibrary.Clamp` (+ _amount _gain) 0 _capacity)))
    (:`then_1`
      (for _array_element _outactors
        (`/Game/Blueprints/Settlement/Settlement.TickGameLogic` _array_element))
      (`self.GatherResources` _outactors))
    (:`then_2`
      (for _array_element_2 _outactors
        (`/Game/Blueprints/Settlement/Settlement.PostTickGamelogic` _array_element_2)))))

(fn `TryPayBlood`
  (params (Amount :type Integer))
  (returns (Success :type Boolean))
  (bind _amount (break `/Game/Blueprints/Gameplay/ResourceState` (`self.BloodResourceState`)))
  (if (<= Amount _amount)
    (setmembers `/Game/Blueprints/Gameplay/ResourceState` :`StructRef` (`self.BloodResourceState`) :`Amount` (- _amount Amount))
    (return true)
    (else
      (return false))))

(fn `UpdateSeason`)

(fn `UserConstructionScript`)